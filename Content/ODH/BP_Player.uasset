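; BP_Player is a player controller Blueprint that steers the controlled pawn toward the mouse cursor.
; BeginPlay adds an Enhanced Input mapping context to the local player.
; Each triggered IA_MouseMove runs a complex Visibility trace under the cursor and, on a blocking hit, caches that point as the destination.
; Follow then applies movement input straight toward it, without pathfinding.
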(event Input|EnhancedActionEvents|EnhancedInputActionIA_MouseMove
  (params (ActionValue :type Boolean) (ElapsedSeconds :type Float%20%28double-precision%29) (TriggeredSeconds :type Float%20%28double-precision%29) (InputAction :type Input%20Action%20Object%20Reference :default "/Game/ODH/IA_MouseMove.IA_MouseMove"))
  (bind (_hit _location) (CallFunction|GetLocationUnderCursor))
  (:Triggered
    (if _hit
      (bind _output_get (Variables|Default|SetCached%20Destination _location))
      (CallFunction|Follow _output_get))))

(event EventBeginPlay
  (Input|AddMappingContext (PlayerController|LocalPlayerSubsystems|GetEnhancedInputLocalPlayerSubsystem (Game|GetPlayerController 0)) "/Game/ODH/IMC_.IMC_" 0 "(bIgnoreAllPressedKeysUntilRelease=True,bForceImmediately=False,bNotifyUserSettings=False)"))

(event Collision|EventActorBeginOverlap
  (params (OtherActor :type Actor%20Object%20Reference)))

(event EventTick
  (params (DeltaSeconds :type Float%20%28single-precision%29)))

(fn ConstructionScript)

(fn GetLocationUnderCursor
  (bind _hitresult (Game|Player|GetHitResultUnderCursorbyChannel "TraceTypeQuery1" true))
  (bind (_bblockinghit _binitialoverlap _time _distance _location) (Collision|BreakHitResult _hitresult))
  (return _bblockinghit _location))

(fn Follow
  (params (Location :type Vector))
  (bind _returnvalue (Pawn|GetControlledPawn))
  (Pawn|Input|AddMovementInput _returnvalue (Math|Vector|GetUnitDirection(Vector) (Transformation|GetActorLocation _returnvalue) Location) 1.0 false))